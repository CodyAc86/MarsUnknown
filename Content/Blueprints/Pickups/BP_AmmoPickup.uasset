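; Ammo pickup actor that refills a BP_Marine's ammo when it overlaps the pickup.
; If the marine's ammo is not full, it plays a reload sound, adds its configured ammo amount and destroys itself.
; Before destruction it decrements the game mode's AmmoSpawned counter, if above zero, keeping the count of spawned pickups in step.
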(event EventBeginPlay)

(event Collision|EventActorBeginOverlap
  (params (OtherActor :type Actor%20Object%20Reference))
  (bind _asbp_marine (Utilities|Casting|CastToBP_Marine OtherActor))
  (if (not (Default|IsAmmoFull _asbp_marine))
    (Utilities|FlowControl|Sequence
      (:then_0
        (Audio|SpawnSound2D "/Game/Sounds/Weapon_AssaultRifle/Stereo/ReloadAudio.ReloadAudio" 1.0 1.0 0.0 0))
      (:then_1
        (Default|AddAmmo _asbp_marine (Variables|Default|GetAmmo%20To%20Add))
        (Utilities|FlowControl|Sequence
          (:then_0
            (bind _asbp_mars_unknown_game_mode (Utilities|Casting|CastToBP_MarsUnknown_GameMode (Game|GetGameMode)))
            (if (> (Variables|/Game/Blueprints/GameMode/BP_MarsUnknown_GameMode.BP_MarsUnknown_GameMode_C|GetAmmoSpawned _asbp_mars_unknown_game_mode) 0)
              (Math|Integer|DecrementInt (Variables|/Game/Blueprints/GameMode/BP_MarsUnknown_GameMode.BP_MarsUnknown_GameMode_C|GetAmmoSpawned _asbp_mars_unknown_game_mode))))
          (:then_1
            (Actor|DestroyActor)))))))

(event EventTick
  (params (DeltaSeconds :type Float%20%28single-precision%29)))

(fn ConstructionScript)