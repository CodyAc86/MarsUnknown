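; BP_MenuGameMode is a menu game mode that shows and hides the options menu widget.
; OpenOptions creates the OptionsMenu widget and adds it to the viewport only when no valid CurrentUI exists, so repeated calls do not stack menus.
; CloseOptionsMenu removes that widget from its parent and clears CurrentUI.
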(event Custom|OpenOptions
  (Utilities|IsValid (Variables|Default|GetCurrentUI)
    (:Is%20Not%20Valid
      (bind _returnvalue (UserInterface|CreateWidget "/Game/UI/OptionsMenu.OptionsMenu_C"))
      (bind _output_get (Variables|Default|SetCurrentUI _returnvalue))
      (UserInterface|Viewport|AddtoViewport _output_get 0))))

(event Custom|CloseOptionsMenu
  (Utilities|IsValid (Variables|Default|GetCurrentUI)
    (:Is%20Valid
      (Widget|RemovefromParent (Variables|Default|GetCurrentUI))
      (Variables|Default|SetCurrentUI 0))))

(event EventBeginPlay)

(event EventTick
  (params (DeltaSeconds :type Float%20%28single-precision%29)))

(fn ConstructionScript)