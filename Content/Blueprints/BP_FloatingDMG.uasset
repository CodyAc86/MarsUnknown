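; Actor that displays a floating damage number in the world through a widget component, then removes itself.
; On BeginPlay it passes its damage amount and crit flag to the W_FloatingDamage widget.
; A timeline lerps the actor from its spawn location to a fixed world-space offset, up and diagonally, and destroys it when finished.
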(event EventBeginPlay
  (bind _asw_floating_damage (Utilities|Casting|CastToW_FloatingDamage (UserInterface|GetWidget (Variables|Default|GetWidget))))
  (Variables|/Game/UI/W_FloatingDamage.W_FloatingDamage_C|SetDmg%20Amt _asw_floating_damage (Variables|Default|GetDamage%20Done))
  (Variables|/Game/UI/W_FloatingDamage.W_FloatingDamage_C|SetIsCrit _asw_floating_damage (Variables|Default|GetIs%20Crit))
  (bind _output_get (Variables|Default|SetStart%20Loc (Transformation|GetActorLocation)))
  (Variables|Default|SetEnd%20Loc (+ _output_get "200.000000,150.000000,200.000000"))
  (bind _move_track (Timeline|Move%20T Play)
    (:Update
      (Transformation|SetActorLocation (Math|Vector|Lerp(Vector) (Variables|Default|GetStart%20Loc) (Variables|Default|GetEnd%20Loc) _move_track) false false))
    (:Finished
      (Actor|DestroyActor))))

(fn ConstructionScript)